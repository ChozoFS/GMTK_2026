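; BP_EnemyDrop is an enemy-drop pickup that takes its name, values, sprite and text from a random data table row at BeginPlay.
; OverlapPowerup triggers UsePowerup and returns the actor so the caller can use it.
; UsePowerup spawns a scan burst, sinks the pickup by ScannedOffset instead of destroying it, and briefly shows its text.
; Respawn and damage logic is disconnected, and several other handlers are empty stubs.
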(event `self.ReceiveBeginPlay`
  (`self.InitializeItemData`))

(event `UsePowerup`
  (bind _returnvalue_location (`KismetMathLibrary.BreakTransform` (`self.GetTransform`)))
  (bind _textrender (`self.TextRender`))
  ; Scanned
  (`NiagaraFunctionLibrary.SpawnSystemAtLocation` "/Game/GMTK-2026/FX/Scan/NE_ScanBurst.NE_ScanBurst" (`SceneComponent.K2_GetComponentLocation` (`self.Sphere`)) (struct) (0.1 0.1 0.1))
  (`SceneComponent.K2_SetWorldLocation` (`self.DefaultSceneRoot`) (+ _returnvalue_location (`KismetMathLibrary.MakeVector` 0.0 0.0 (* (`self.ScannedOffset`) -1.0))) false false)
  (`TextRenderComponent.K2_SetText` _textrender (`self.Text to Show`))
  (`KismetSystemLibrary.Delay` 1.5)
  ;; Code will need to be changed for 1 time pickups
  (`TextRenderComponent.K2_SetText` _textrender (`KismetTextLibrary.Conv_StringToText` "")))

(event `InitializeItemData`
  (bind _outrownames (`DataTableFunctionLibrary.GetDataTableRowNames` (`self.DropsDataTable`)))
  (bind _returnvalue (`|GetDataTableRow` "/Game/Pickups/DT_EnemyDrops.DT_EnemyDrops" (`KismetArrayLibrary.Array_Random` _outrownames))
    (:`then`
      (set `self.CurrentData` _returnvalue)
      (bind (_powerupname _scorevalue _timevalue _duration _genericincrease _sprite _texttoshow) (break `/Game/Pickups/Struct_EnemyDrop` _returnvalue))
      (set `self.Item Name` _powerupname)
      (set `self.ScoreValue` _scorevalue)
      (set `self.Time Value` _timevalue)
      (set `self.Duration` _duration)
      (set `self.Generic Increase` _genericincrease)
      (`PaperSpriteComponent.SetSprite` (`self.PaperSprite`) _sprite)
      (set `self.Text to Show` _texttoshow))
    (:`RowNotFound`
      (`KismetSystemLibrary.PrintString` "PICKUP ITEM TRYING TO INITIALIZE WITH NO DATA ROW"))))

(event `self.SendHit`
  (params (Direction :type "Vector Structure")))

(event `SetDamagedState`
  (params (NewState :type Boolean)))

(event `/Game/GMTK-2026/Blueprints/BPI_Combat.StunPlayer`
  (params (Direction :type "Vector Structure")))

(event `self.Sphere.OnComponentBeginOverlap`
  (params (OverlappedComponent :type "PrimitiveComponent Object Reference") (OtherActor :type "Actor Object Reference") (OtherComp :type "PrimitiveComponent Object Reference") (OtherBodyIndex :type Integer) (bFromSweep :type Boolean) (SweepResult :type "HitResult Structure (by ref)")))

(fn `OverlapPowerup`
  (returns (NewParam :type "/Game/Pickups/BP_EnemyDrop Object Reference"))
  (`self.UsePowerup`)
  (return self))

(fn `ReturnEnemyBP`
  (returns (EnemyScanned :type "/Game/GMTK-2026/Blueprints/Enemies/BP_Base_Enemy Object Reference"))
  (return null))

(fn `ScanItem`
  (returns (ItemToPickup :type "/Game/Pickups/BP_BasePickup Object Reference"))
  (return null))

(fn `UserConstructionScript`
  (`StaticMeshComponent.SetStaticMesh` (`self.StaticMesh`) (`self.ItemMesh`)))