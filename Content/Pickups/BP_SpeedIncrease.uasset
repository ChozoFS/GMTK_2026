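; Speed boost pickup Blueprint that overrides a parent powerup's activate and deactivate functions to temporarily raise the player's movement speed.
; Activation sets the player's boost flag and modifier, then passes current max speed multiplied by the modifier to UpdateMovementSpeed.
; Deactivation clears the flag and divides the then-current max speed by the modifier, rather than restoring a saved base value.
; Both functions print debug strings, and the event graph has no active logic.
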(fn `ActivatePowerup`
  (params (Player :type "/Game/GMTK-2026/Blueprints/BP_Character2D Object Reference"))
  (bind _speedboostmodifier (`self.SpeedBoostModifier`))
  (bind _returnvalue (`MovementComponent.GetMaxSpeed` (`Pawn.GetMovementComponent` Player)))
  (`parent.ActivatePowerup` Player)
  (bind _output_get (set `/Game/GMTK-2026/Blueprints/BP_Character2D.SpeedBoostActive` true Player))
  (set `/Game/GMTK-2026/Blueprints/BP_Character2D.SpeedBoostModifier` _speedboostmodifier Player)
  (`KismetSystemLibrary.PrintString` (`KismetStringLibrary.Concat_StrStr` (`KismetStringLibrary.Conv_BoolToString` _output_get) " - " (`KismetStringLibrary.Conv_DoubleToString` _returnvalue)))
  (`/Game/GMTK-2026/Blueprints/BP_Character2D.UpdateMovementSpeed` Player (* _speedboostmodifier _returnvalue)))

(fn `DeactivatePowerup`
  (params (PlayerBP :type "/Game/GMTK-2026/Blueprints/BP_Character2D Object Reference"))
  (bind _returnvalue (/ (`MovementComponent.GetMaxSpeed` (`Pawn.GetMovementComponent` PlayerBP)) (`self.SpeedBoostModifier`)))
  (`parent.DeactivatePowerup` PlayerBP)
  (set `/Game/GMTK-2026/Blueprints/BP_Character2D.SpeedBoostActive` false PlayerBP)
  (`/Game/GMTK-2026/Blueprints/BP_Character2D.UpdateMovementSpeed` PlayerBP _returnvalue)
  (`KismetSystemLibrary.PrintString` (`KismetStringLibrary.Conv_DoubleToString` _returnvalue)))

(fn `UserConstructionScript`
  (`parent.UserConstructionScript`))