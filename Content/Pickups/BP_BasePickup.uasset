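; Base pickup actor that takes its name, score value, sprite and damaged state from a random data table row at BeginPlay.
; Scanning returns the pickup, spawns a Niagara burst, drops it by an offset, then re-rolls its data after a delay and raises it back, recycling the same actor.
; A hit marks it damaged and applies that row's tint to the sprite.
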(event `self.ReceiveBeginPlay`
  (`self.InitializeItemData`))

(event `Scanned`
  (bind _returnvalue_location (`KismetMathLibrary.BreakTransform` (`self.GetTransform`)))
  (bind _defaultsceneroot (`self.DefaultSceneRoot`))
  ; Scanned
  (`NiagaraFunctionLibrary.SpawnSystemAtLocation` "/Game/GMTK-2026/FX/Scan/NE_ScanBurst.NE_ScanBurst" (`SceneComponent.K2_GetComponentLocation` (`self.Sphere`)) (struct) (0.1 0.1 0.1))
  (`SceneComponent.K2_SetWorldLocation` _defaultsceneroot (+ _returnvalue_location (`KismetMathLibrary.MakeVector` 0.0 0.0 (* (`self.ScannedOffset`) -1.0))) false false)
  (`KismetSystemLibrary.Delay` 1.5)
  (`self.InitializeItemData`)
  (`SceneComponent.K2_SetWorldLocation` _defaultsceneroot (+ _returnvalue_location (`KismetMathLibrary.MakeVector` 0.0 0.0 (`self.ScannedOffset`))) false false))

(event `InitializeItemData`
  (bind _outrownames (`DataTableFunctionLibrary.GetDataTableRowNames` (`self.PickupDataTable`)))
  (bind _returnvalue (`|GetDataTableRow` "/Game/Pickups/DT_Pickups.DT_Pickups" (`KismetArrayLibrary.Array_Random` _outrownames))
    (:`then`
      (set `self.CurrentData` _returnvalue)
      (bind (_itemname _isdamaged _scorevalue _sprite) (break `/Game/Pickups/Struct_Pickup` _returnvalue))
      (set `self.Item Name` _itemname)
      (`self.SetDamagedState` _isdamaged)
      (set `self.ScoreValue` _scorevalue)
      (`PaperSpriteComponent.SetSprite` (`self.PaperSprite`) _sprite))
    (:`RowNotFound`
      (`KismetSystemLibrary.PrintString` "PICKUP ITEM TRYING TO INITIALIZE WITH NO DATA ROW"))))

(event `/Game/GMTK-2026/Blueprints/BPI_Combat.SendHit`
  (params (Direction :type "Vector Structure"))
  (if (not (`self.Damaged`))
    (`self.SetDamagedState` true)))

(event `SetDamagedState`
  (params (NewState :type Boolean))
  (bind _papersprite (`self.PaperSprite`))
  (bind (_currentdata_itemname _currentdata_isdamaged _currentdata_scorevalue _currentdata_sprite _currentdata_damagedtint) (break `/Game/Pickups/Struct_Pickup` (`self.CurrentData`)))
  (if NewState
    (set `self.Damaged` true)
    (`PaperSpriteComponent.SetSpriteColor` _papersprite _currentdata_damagedtint)
    (else
      (set `self.Damaged` false)
      (`PaperSpriteComponent.SetSpriteColor` _papersprite (struct :`R` 1.0 :`G` 1.0 :`B` 1.0 :`A` 1.0)))))

(fn `ScanItem`
  (returns (ItemToPickup :type "/Game/Pickups/BP_BasePickup Object Reference"))
  (`self.Scanned`)
  (return self))

(fn `UserConstructionScript`
  (`StaticMeshComponent.SetStaticMesh` (`self.StaticMesh`) (`self.ItemMesh`)))