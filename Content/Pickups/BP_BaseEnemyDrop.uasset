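; Base pickup for enemy drops, with sprite, popup text and duration loaded from a DT_EnemyDrops row during construction.
; A player-tagged overlap fires once, spawning VFX and sound, shifting the root by ScannedOffset and detaching text that a timeline raises, scales and fades through a dynamic material.
; It then calls ActivatePowerup, waits for the duration and calls DeactivatePowerup, both empty here.
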(event `self.ReceiveBeginPlay`
  (bind _textrender (`self.TextRender`))
  (bind _returnvalue (`KismetMaterialLibrary.CreateDynamicMaterialInstance` (`TextRenderComponent.TextMaterial` _textrender)))
  (bind _output_get (set `self.CustomTextMaterial` _returnvalue))
  (`TextRenderComponent.SetTextMaterial` _textrender _output_get))

(event `UsePowerup`
  (bind _textrender (`self.TextRender`))
  (bind _textrender_2 (`self.TextRender`))
  (bind _returnvalue (`SceneComponent.K2_GetComponentLocation` (`self.TextRender`)))
  ; Spawns VFX + Set Text
  (`NiagaraFunctionLibrary.SpawnSystemAtLocation` (`self.PickupVFX`) (`SceneComponent.K2_GetComponentLocation` (`self.Sphere`)) (struct) (0.1 0.1 0.1) true true "AutoRelease")
  (`GameplayStatics.PlaySound2D` (`self.PickupSound`) 1.0 1.0 0.0 null null)
  (`SceneComponent.K2_DetachFromComponent` (`self.TextRender`) "KeepWorld" "KeepRelative" "KeepRelative" true)
  (bind _returnvalue_2 (`self.CalculateMoveToPosition`))
  (`SceneComponent.K2_SetWorldLocation` (`self.DefaultSceneRoot`) _returnvalue_2 false false)
  (`TextRenderComponent.K2_SetText` _textrender_2 (`self.Text to Show`))
  (bind (_direction _newtrack_0 _fade _grow) (`Timeline|Timeline_0`) ; Make sure track length is same as text lifetime
    (:`Update`
      (`MaterialInstanceDynamic.SetScalarParameterValue` (`self.CustomTextMaterial`) "Opacity" _fade)
      (`SceneComponent.K2_SetWorldLocation` (`self.TextRender`) (`KismetMathLibrary.VLerp` _returnvalue (+ _returnvalue (0.0 0.0 5.0)) _newtrack_0) false false)
      (`TextRenderComponent.SetWorldSize` _textrender (* _grow (`TextRenderComponent.WorldSize` _textrender))))
    (:`Finished`
      (`TextRenderComponent.K2_SetText` _textrender_2 (`KismetTextLibrary.Conv_StringToText` "")))))

(event `ResetDoOnce`
  (goto _label :!via `Reset`))

(event `self.Sphere.OnComponentBeginOverlap`
  (params (OverlappedComponent :type "PrimitiveComponent Object Reference") (OtherActor :type "Actor Object Reference") (OtherComp :type "PrimitiveComponent Object Reference") (OtherBodyIndex :type Integer) (bFromSweep :type Boolean) (SweepResult :type "HitResult Structure (by ref)"))
  (if (`self.ActorHasTag` OtherActor "Player")
    (`/Engine/EditorBlueprintResources/StandardMacros.DoOnce` false :!label _label
      (:`Completed`
        (`self.UsePowerup`)
        (bind _player (message `/Game/GMTK-2026/Blueprints/BPI_Combat.ReturnPlayerRef` OtherActor))
        (bind _output_get (set `self.Player` _player))
        (`self.ActivatePowerup` _output_get)
        (`KismetSystemLibrary.Delay` (`self.Duration`))
        (`self.DeactivatePowerup` (`self.Player`))))))

(fn `ActivatePowerup`
  (params (Player :type "/Game/GMTK-2026/Blueprints/BP_Character2D Object Reference")))

(fn `CalculateMoveToPosition`
  (returns (ReturnValue :type "Vector Structure"))
  (bind _returnvalue_location (`KismetMathLibrary.BreakTransform` (`self.GetTransform`)))
  (return (+ _returnvalue_location (`KismetMathLibrary.MakeVector` 0.0 0.0 (* (`self.ScannedOffset`) -1.0)))))

(fn `DeactivatePowerup`
  (params (PlayerBP :type "/Game/GMTK-2026/Blueprints/BP_Character2D Object Reference")))

(fn `ReturnEnemyBP`
  (returns (EnemyScanned :type "/Game/GMTK-2026/Blueprints/Enemies/BP_Base_Enemy Object Reference"))
  (return null))

(fn `ReturnPlayerRef`
  (returns (Player :type "/Game/GMTK-2026/Blueprints/BP_Character2D Object Reference"))
  (return null))

(fn `ReturnStruct`
  (returns (PickupDeets :type "/Game/Pickups/Struct_Pickup Structure") (EnemyDeets :type "/Game/GMTK-2026/Blueprints/Enemies/Struct_EnemyDetails Structure"))
  (return))

(fn `ScanItem`
  (returns (ItemToPickup :type "/Game/Pickups/BP_BasePickup Object Reference"))
  (return null))

(fn `UserConstructionScript`
  (bind (_datatablerowhandle_datatable _datatablerowhandle_rowname) (break `DataTableRowHandle` (`self.DataTableRowHandle`)))
  (bind _returnvalue (`|GetDataTableRow` "/Game/Pickups/DT_EnemyDrops.DT_EnemyDrops" _datatablerowhandle_rowname)
    (:`then`
      (set `self.CurrentData` _returnvalue)
      (bind (_powerupname _sprite _texttoshow _duration) (break `/Game/Pickups/Struct_EnemyDrop` _returnvalue))
      (set `self.Item Name` _powerupname)
      (`PaperSpriteComponent.SetSprite` (`self.PaperSprite`) _sprite)
      (set `self.Text to Show` _texttoshow)
      (`self.ResetDoOnce`)
      (set `self.Duration` _duration))
    (:`RowNotFound`
      (`KismetSystemLibrary.PrintString` "PICKUP ITEM TRYING TO INITIALIZE WITH NO DATA ROW" true true (struct :`R` 1.0 :`G` 0.012118 :`A` 1.0) 5.0))))