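; Enemy-drop pickup Blueprint that grants the player a rapid-fire powerup.
; It overrides the parent's ActivatePowerup to cache the player's TimeBetweenShots, then divide it by ShotSpeedMultiplier.
; DeactivatePowerup calls the parent and restores the cached value.
; The event graph holds only disabled placeholder events, so all behavior lives in these two overrides and the inherited parent logic.
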(fn `ActivatePowerup`
  (params (Player :type "/Game/GMTK-2026/Blueprints/BP_Character2D Object Reference"))
  (bind _timebetweenshots (`/Game/GMTK-2026/Blueprints/BP_Character2D.TimeBetweenShots` Player))
  (`parent.ActivatePowerup` Player)
  (set `self.OriginalTimeBetweenShots` _timebetweenshots)
  (set `/Game/GMTK-2026/Blueprints/BP_Character2D.TimeBetweenShots` (* _timebetweenshots (/ 1.0 (`self.ShotSpeedMultiplier`))) Player))

(fn `DeactivatePowerup`
  (params (PlayerBP :type "/Game/GMTK-2026/Blueprints/BP_Character2D Object Reference"))
  (`parent.DeactivatePowerup` PlayerBP)
  (set `/Game/GMTK-2026/Blueprints/BP_Character2D.TimeBetweenShots` (`self.OriginalTimeBetweenShots`) PlayerBP))

(fn `UserConstructionScript`
  (`parent.UserConstructionScript`))