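; Actor component that marks an object as belonging to an object pool and lets it return itself to that pool.
; Init stores the owning pool and starts the object inactive.
; RecycleSelf hands the component back to the pool, and OnDeactivated triggers the same recycle.
; EndPlay unbinds from the pool's cleanup event.
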(event `self.ReceiveBeginPlay`)

(event `self.ReceiveEndPlay`
  (params (EndPlayReason :type "EEndPlayReason Enum" :default "Destroyed"))
  (remove `/Game/GMTK-2026/Blueprints/BP_ObjectPool.OnPoolerCleanup` (`self.ObjectPool`) (`|CreateDelegate` :!event `RecycleSelf`)))

(fn `Init`
  (params (Owner :type "/Game/GMTK-2026/Blueprints/BP_ObjectPool Object Reference"))
  (set `self.isActive?` false)
  (set `self.ObjectPool` Owner))

(fn `OnDeactivated`
  (`self.RecycleSelf`))

(fn `RecycleSelf`
  ; Call Recycle Pooled Object from Object Pool
  (`/Game/GMTK-2026/Blueprints/BP_ObjectPool.RecyclePooledObject` (`self.ObjectPool`) self))