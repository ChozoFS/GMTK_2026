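; Actor object pool that pre-spawns configured actor types on BeginPlay and hands them out by type enum for reuse.
; Each actor gets an AC_PooledObject component tracking active state; idle actors are hidden, stripped of collision and tick, and attached to the pool.
; GetPooledActor activates and notifies a free actor, regenerates invalid entries, or grows pools allowing it.
; Recycle functions deactivate actors, and a cleanup dispatcher is bound on handout.
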(event `self.ReceiveBeginPlay`
  (`parent.ReceiveBeginPlay`)
  (`self.Setup`))

(fn `BroadcastPoolerCleanup`
  (`self.OnPoolerCleanup`))

(fn `GetPooledActor`
  (params (`Object Type` :type "/Game/GMTK-2026/Blueprints/E_PooledObjectTypes Enum" :default "NewEnumerator0") (DesiredSpawnLocation :type "Vector Structure") (DesiredSpawnRotation :type "Rotator Structure") (UseCustomSpawnLocationAndRotation :type Boolean))
  (returns (PooledActor :type "Actor Object Reference"))
  (locals (PoolCount :type Integer) (CurrentPool :type Integer :default -1) (PooledObjectCount :type Integer) (FirstAvailable :type Integer :default -1) (ToReturn :type "/Game/GMTK-2026/Blueprints/AC_PooledObject Object Reference") (ToReturnActor :type "Actor Object Reference") (SpawnedActor :type "Actor Object Reference") (PoolComponent :type "/Game/GMTK-2026/Blueprints/AC_PooledObject Object Reference") (ReturnLocation :type "Vector Structure") (ReturnRotation :type "Rotator Structure") (UseCustomLocationAndRotation :type Boolean))
  (bind _poolcomponent (`local.PoolComponent`))
  (bind _spawnedactor (`local.SpawnedActor`))
  (bind _output (`|GetArrayItem` (`self.Pools`) (`local.CurrentPool`)))
  (bind (_actortemplate _poolsize _cangrow) (break `/Game/GMTK-2026/Blueprints/Structs/S_PooledObjectData` (`|GetArrayItem` (`self.PooledObjectData`) (`local.CurrentPool`))))
  (bind _pooledobjects (break `/Game/GMTK-2026/Blueprints/Structs/S_SingleObjectPool` _output))
  (set `local.UseCustomLocationAndRotation` UseCustomSpawnLocationAndRotation)
  (set `local.ReturnLocation` DesiredSpawnLocation)
  (set `local.ReturnRotation` DesiredSpawnRotation)
  (bind _output_get (set `local.PoolCount` (`KismetArrayLibrary.Array_Length` (`self.Pools`))))
  (for _index (range _output_get)
    ;[0.15 0.15 0.15 0.5 30] This is ugly, but all its doing is saying if we find the element we're looking for, stop looping
    (if (`|EnumEquality` `Object Type` (`.ActorEnum_15_C0724C5E4BA7DCCB7B1E738BBF8AC11B` (break `/Game/GMTK-2026/Blueprints/Structs/S_PooledObjectData` (`|GetArrayItem` (`self.PooledObjectData`) _index))))
      (set `local.CurrentPool` _index)
      (break)))
  (if (== (`local.CurrentPool`) -1)
    (return null)
    (else
      ;[0.15 0.15 0.15 0.5 50] Pool Found
      (set `local.PooledObjectCount` (`KismetArrayLibrary.Array_Length` (`.PooledObjects_3_2B03F95A4B239BBF05F6229CE2736506` (break `/Game/GMTK-2026/Blueprints/Structs/S_SingleObjectPool` (`|GetArrayItem` (`self.Pools`) (`local.CurrentPool`))))))
      (for _index_2 (range (+ (- (`local.PooledObjectCount`) -1) 1))
        (bind _output_2 (`|GetArrayItem` (`.PooledObjects_3_2B03F95A4B239BBF05F6229CE2736506` (break `/Game/GMTK-2026/Blueprints/Structs/S_SingleObjectPool` (`|GetArrayItem` (`self.Pools`) (`local.CurrentPool`)))) _index_2))
        (if (`KismetSystemLibrary.IsValid` _output_2)
          (if (not (`/Game/GMTK-2026/Blueprints/AC_PooledObject.isActive?` _output_2))
            (set `local.FirstAvailable` _index_2)
            (break))
          (else
            (`self.RegenItem` (`local.CurrentPool`) _index_2)
            (break))))
      (if (>= (`local.FirstAvailable`) 0)
        ;[0.15 0.15 0.15 0.5 50] Object Available
        (bind _output_get_2 (set `local.ToReturn` (`|GetArrayItem` (`.PooledObjects_3_2B03F95A4B239BBF05F6229CE2736506` (break `/Game/GMTK-2026/Blueprints/Structs/S_SingleObjectPool` (`|GetArrayItem` (`self.Pools`) (`local.CurrentPool`)))) (`local.FirstAvailable`))))
        (set `/Game/GMTK-2026/Blueprints/AC_PooledObject.isActive?` true _output_get_2)
        (set `local.ToReturnActor` (`ActorComponent.GetOwner` _output_get_2))
        (`self.SetActorHiddenInGame` (`local.ToReturnActor`) false)
        (`self.SetActorEnableCollision` (`local.ToReturnActor`) true)
        (`self.SetActorTickEnabled` (`local.ToReturnActor`) true)
        (`self.K2_AttachToActor` (`local.ToReturnActor`) null "None" "SnapToTarget" "SnapToTarget" "KeepRelative" true)
        (if (`local.UseCustomLocationAndRotation`)
          (`self.K2_SetActorLocation` (`local.ToReturnActor`) (`local.ReturnLocation`) false false)
          (`self.K2_SetActorRotation` (`local.ToReturnActor`) (`local.ReturnRotation`) false))
        (message `/Game/GMTK-2026/Blueprints/BPI_Poolable.OnActivatedFromPool` (`local.ToReturnActor`))
        (add `self.OnPoolerCleanup` (`|CreateDelegate` (`local.ToReturn`) :!event `RecycleSelf`))
        (return (`local.ToReturnActor`))
        (else
          ;[0.15 0.15 0.15 0.5 50] Out Of Room Need To Grow
          (if (not _cangrow)
            (return null)
            (else
              (bind _returnvalue (`|SpawnActorFromClass` _actortemplate (`KismetMathLibrary.MakeTransform` (0.0 0.0 0.0)) "AlwaysSpawn" "MultiplyWithRoot" null null))
              (bind _output_get_3 (set `local.SpawnedActor` _returnvalue))
              (bind _returnvalue_2 (`AddComponent|NODE_AddAC_PooledObject-1` :`self` _output_get_3))
              (bind _output_get_4 (set `local.PoolComponent` _returnvalue_2))
              (`/Game/GMTK-2026/Blueprints/AC_PooledObject.Init` _output_get_4 self)
              (`KismetArrayLibrary.Array_Add` _pooledobjects _poolcomponent)
              (setmembers `/Game/GMTK-2026/Blueprints/Structs/S_SingleObjectPool` :`StructRef` _output :`PooledObjects` _pooledobjects)
              (set `/Game/GMTK-2026/Blueprints/AC_PooledObject.isActive?` true _poolcomponent)
              (add `self.OnPoolerCleanup` (`|CreateDelegate` (`local.PoolComponent`) :!event `RecycleSelf`))
              (message `/Game/GMTK-2026/Blueprints/BPI_Poolable.OnActivatedFromPool` _spawnedactor)
              (return _spawnedactor))))))))

(fn `RecycleActor`
  (params (PooledActor :type "Actor Object Reference"))
  (locals (PoolComponentRef :type "/Game/GMTK-2026/Blueprints/AC_PooledObject Object Reference"))
  (bind _returnvalue (`self.GetComponentByClass` PooledActor "/Game/GMTK-2026/Blueprints/AC_PooledObject.AC_PooledObject_C"))
  (`/Engine/EditorBlueprintResources/StandardMacros.IsValid` _returnvalue
    (:`Is Valid`
      (`self.RecyclePooledObject` _returnvalue))))

(fn `RecyclePooledObject`
  (params (PoolComponent :type "/Game/GMTK-2026/Blueprints/AC_PooledObject Object Reference"))
  (locals (ReturningActor :type "Actor Object Reference"))
  (set `/Game/GMTK-2026/Blueprints/AC_PooledObject.isActive?` false PoolComponent)
  (bind _output_get (set `local.ReturningActor` (`ActorComponent.GetOwner` PoolComponent)))
  (`self.SetActorHiddenInGame` _output_get true)
  (`self.SetActorEnableCollision` (`local.ReturningActor`) false)
  (`self.SetActorTickEnabled` (`local.ReturningActor`) false)
  (`self.K2_AttachToActor` (`local.ReturningActor`) self "None" "SnapToTarget" "SnapToTarget" "KeepRelative" true))

(fn `RegenItem`
  (params (PoolIndex :type Integer) (PositionIndex :type Integer))
  (locals (SpawnedActor :type "Actor Object Reference"))
  (bind _output (`|GetArrayItem` (`self.Pools`) PoolIndex))
  (bind _pooledobjects (break `/Game/GMTK-2026/Blueprints/Structs/S_SingleObjectPool` _output))
  (bind _returnvalue (`|SpawnActorFromClass` (`.ActorTemplate_2_EA250FBF4C812FAF27B929A92004C8D7` (break `/Game/GMTK-2026/Blueprints/Structs/S_PooledObjectData` (`|GetArrayItem` (`self.PooledObjectData`) PoolIndex))) (`KismetMathLibrary.MakeTransform` (0.0 0.0 0.0)) "AlwaysSpawn" "MultiplyWithRoot" null null))
  (bind _output_get (set `local.SpawnedActor` _returnvalue))
  (bind _returnvalue_2 (`AddComponent|NODE_AddAC_PooledObject-2` :`self` _output_get))
  (`/Game/GMTK-2026/Blueprints/AC_PooledObject.Init` _returnvalue_2 null)
  (`KismetArrayLibrary.Array_Insert` _pooledobjects _returnvalue_2 PositionIndex)
  (setmembers `/Game/GMTK-2026/Blueprints/Structs/S_SingleObjectPool` :`StructRef` _output :`PooledObjects` _pooledobjects)
  (`self.SetActorHiddenInGame` (`local.SpawnedActor`) true)
  (`self.SetActorEnableCollision` (`local.SpawnedActor`) false)
  (`self.SetActorTickEnabled` (`local.SpawnedActor`) false)
  (`self.K2_AttachToActor` (`local.SpawnedActor`) self "None" "SnapToTarget" "SnapToTarget" "KeepRelative" true))

(fn `Setup`
  (locals (CurrentPool :type "/Game/GMTK-2026/Blueprints/Structs/S_SingleObjectPool Structure") (PoolComponent :type "/Game/GMTK-2026/Blueprints/AC_PooledObject Object Reference") (SpawnedActor :type "Actor Object Reference"))
  (bind _pooledobjectdata (`self.PooledObjectData`))
  (bind _currentpool (`local.CurrentPool`))
  (bind _pooledobjects (break `/Game/GMTK-2026/Blueprints/Structs/S_SingleObjectPool` _currentpool))
  (for _index (range (+ (`KismetArrayLibrary.Array_Length` _pooledobjectdata) 1))
    (set `local.CurrentPool` (struct))
    (bind (_actortemplate _poolsize) (break `/Game/GMTK-2026/Blueprints/Structs/S_PooledObjectData` (`|GetArrayItem` _pooledobjectdata _index)))
    (for _ (range _poolsize)
      (bind _returnvalue (`|SpawnActorFromClass` _actortemplate (`KismetMathLibrary.MakeTransform` (0.0 0.0 0.0)) "AlwaysSpawn" "MultiplyWithRoot" null null))
      (bind _output_get (set `local.SpawnedActor` _returnvalue))
      (bind _returnvalue_2 (`AddComponent|NODE_AddAC_PooledObject-0` :`self` _output_get))
      (bind _output_get_2 (set `local.PoolComponent` _returnvalue_2))
      (`/Game/GMTK-2026/Blueprints/AC_PooledObject.Init` _returnvalue_2 self)
      (`/Game/GMTK-2026/Blueprints/AC_PooledObject.Init` _output_get_2 self)
      (`KismetArrayLibrary.Array_Add` _pooledobjects (`local.PoolComponent`))
      (setmembers `/Game/GMTK-2026/Blueprints/Structs/S_SingleObjectPool` :`StructRef` _currentpool :`PooledObjects` _pooledobjects)
      (`self.SetActorHiddenInGame` (`local.SpawnedActor`) true)
      (`self.SetActorEnableCollision` (`local.SpawnedActor`) false)
      (`self.SetActorTickEnabled` (`local.SpawnedActor`) false)
      (`self.K2_AttachToActor` (`local.SpawnedActor`) self "None" "SnapToTarget" "SnapToTarget" "KeepRelative" true))
    (`KismetArrayLibrary.Array_Add` (`self.Pools`) (`local.CurrentPool`))))

(fn `UserConstructionScript`)