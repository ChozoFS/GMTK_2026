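; Player 2D flipbook character that shoots pooled lasers and scans items and enemies for score and money.
; Tick aims the scanner at the cursor, eases a detached camera toward it, shows hovered details and picks animation states without a state machine.
; Holding scan slows movement and sweeps a sphere trace, buying pickups or cashing in stunned enemies through BPI_Combat.
; Enemy hits take money, knock back and briefly stun.
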(event Custom|ChangeAnimFlipbooks
  (params (Desired%20Anim%20State :type E_AnimState%20Enum :default "E_AnimState_MAX"))
  (bind _sprite (Variables|Default|GetSprite))
  ;[0 0.117 0.15] Character Animation Stuff
  ;;[0.02382 1 0.7369 0.5] Change Flipbook Animation
  (bind _output_get (Variables|Default|SetAnim%20State Desired%20Anim%20State))
  (if (!= (Class|PaperFlipbookComponent|GetFlipbook _sprite) (Utilities|Select :Index _output_get :NewEnumerator0 "/Game/NoahTest/SPR_Hero_Idle_Flipbook.SPR_Hero_Idle_Flipbook" :NewEnumerator1 "/Game/NoahTest/PlayerWalkRight.PlayerWalkRight" :NewEnumerator2 "/Game/NoahTest/SPR_Hero_Hurt_Flipbook.SPR_Hero_Hurt_Flipbook"))
    (Sprite|SetFlipbook _sprite (Utilities|Select :Index _output_get :NewEnumerator0 "/Game/NoahTest/SPR_Hero_Idle_Flipbook.SPR_Hero_Idle_Flipbook" :NewEnumerator1 "/Game/NoahTest/PlayerWalkRight.PlayerWalkRight" :NewEnumerator2 "/Game/NoahTest/SPR_Hero_Hurt_Flipbook.SPR_Hero_Hurt_Flipbook"))))

(event Custom|ScanAnimFinished
  ;[0.02718 1 0 0.5 50] Begin Play
  (Development|SetHiddeninGame (Variables|Default|GetScanAnim) true false))

(event Custom|DetermineCurrentAnimState
  (bind _dustparticle (Variables|Default|GetDustParticle))
  ;[0 0.117 0.15] Character Animation Stuff
  ;;[0.002416 1 0.2753 0.5] Per Tick, determine proper animation state
  ;;;[0.15 0.15 0.15 0.5] Because there's no state machine I gotta do this shit
  (if (not (Variables|Default|GetStunned?))
    (if (!= (Math|Vector|VectorLength (Variables|/Script/Engine.MovementComponent|GetVelocity (Variables|Character|GetCharacterMovement))) 0.0)
      (CallFunction|ChangeAnimFlipbooks "NewEnumerator1")
      ;;[0.15 0.15 0.15 0.5] Activate Dust Particles if walking and not scanning
      (if (or (Variables|Default|GetScanning?) (Variables|Default|GetStunned?))
        (Components|Activation|Deactivate _dustparticle)
        (else
          (Components|Activation|Activate _dustparticle false)))
      (else
        (CallFunction|ChangeAnimFlipbooks "NewEnumerator0")
        (Components|Activation|Deactivate _dustparticle)))
    (else
      (CallFunction|ChangeAnimFlipbooks "NewEnumerator2"))))

(event Custom|Knockback
  (params (Direction :type Vector))
  (bind _returnvalue (* Direction 1.5e+03))
  (bind (_x _y) (Math|Vector|BreakVector _returnvalue))
  ;[0.15 0.15 0.15 0.5] Player knockback
  (Utilities|FlowControl|DoOnce false :!label _label
    (:Completed
      (Character|LaunchCharacter (Math|Vector|MakeVector _x _y 1e+02) true true)
      (Variables|Default|SetStunned? true)
      (Utilities|FlowControl|Sequence
        (:then_0
          (Audio|PlaySound2D "/Game/Sound/SFX/SFX_PlayerHurt.SFX_PlayerHurt" 1.0 1.0 0.0 0 0))
        (:then_1
          (Utilities|FlowControl|Delay 2.0)
          (Variables|Default|SetStunned? false)
          (goto _label Reset))))))

(event Input|EnhancedActionEvents|EnhancedInputActionIA_Move
  (params (ActionValue :type Vector%202D%20Structure) (ElapsedSeconds :type Float%20%28double-precision%29) (TriggeredSeconds :type Float%20%28double-precision%29) (InputAction :type Input%20Action%20Object%20Reference :default "/Game/GMTK-2026/Input/Actions/IA_Move.IA_Move"))
  (bind (_x _y) (Math|Vector2D|BreakVector2D ActionValue))
  (bind _startingscale (Variables|Default|GetStartingScale))
  (bind (_x_2 _y_2 _z) (Math|Vector|BreakVector _startingscale))
  ;[0.15 0.15 0.15 0.5 50] Input Actions
  ;;[0 0.489 1 0.5 30] WASD Movement
  (Utilities|FlowControl|Sequence
    (:then_0
      (if (not (Variables|Default|GetStunned?))
        (Pawn|Input|AddMovementInput "1.000000,0.000000,0.000000" _x false)
        (Pawn|Input|AddMovementInput "0.000000,1.000000,0.000000" _y false)
        (if (< _y 0.0)
          ;;;[0 0.489 1 0.5 22] Flip Sprite Depending on Movment Direction
          (bind _result (Math|Float|NegateFloat _x_2)
            (:%20%20
              (Transformation|SetRelativeScale3D (Variables|Default|GetSprite) (Math|Vector|MakeVector _result _y_2 _z))))
          (else
            ;;;;[0 0.489 1 0.5] Prevents flipping on input release
            (if (> _y 0.0)
              (Transformation|SetRelativeScale3D (Variables|Default|GetSprite) (Variables|Default|GetStartingScale)))))))
    (:then_1
      (Variables|Default|SetAbsMoveInput (Math|Float|Absolute(Float) (+ _x _y))))))

(event Input|EnhancedActionEvents|EnhancedInputActionIA_Scan
  (params (ActionValue :type Vector%202D%20Structure) (ElapsedSeconds :type Float%20%28double-precision%29) (TriggeredSeconds :type Float%20%28double-precision%29) (InputAction :type Input%20Action%20Object%20Reference :default "/Game/GMTK-2026/Input/Actions/IA_Scan.IA_Scan"))
  (bind _timerbp (Variables|Default|GetTimerBP))
  (bind _anim_state (Variables|Default|GetAnim%20State))
  (bind _sprite (Variables|Default|GetSprite))
  (bind _timerbp_2 (Variables|Default|GetTimerBP))
  (bind _returnvalue (Utilities|Enum|Equal(Enum) _anim_state "NewEnumerator1"))
  ;[0.15 0.15 0.15 0.5 50] Input Actions
  ;;[0 0.489 1 0.5 30] Scanning Logic
  (:Triggered
    (if (not (Variables|Default|GetStunned?))
      (bind _output_get (Variables|Default|SetScanAlpha (Math|Float|Fraction (+ (Variables|Default|GetScanAlpha) (/ (Variables|Default|GetDelta%20Seconds) (Class|PaperFlipbookComponent|GetFlipbookLength (Variables|Default|GetScanAnim)))))))
      (bind _spheretraceend (CallFunction|CalculateSphereTraceEnd))
      (bind _spheretracestart (CallFunction|CalculateShotStartingPos))
      (bind (_outhit _returnvalue_2) (Class|KismetSystemLibrary|SphereTraceSinglebyProfile _spheretracestart (Math|Vector|Lerp(Vector) _spheretracestart _spheretraceend _output_get) 65.0 "None" false 0 "None" true "(R=1.000000,G=0.000000,B=0.000000,A=1.000000)" "(R=0.000000,G=1.000000,B=0.000000,A=1.000000)" (Class|PaperFlipbookComponent|GetFlipbookLength (Variables|Default|GetScanAnim))))
      (if _returnvalue_2
        (if (Utilities|DoesObjectImplementInterface (.hitactor _outhit) "/Game/GMTK-2026/Blueprints/BPI_Combat.BPI_Combat_C")
          (if (Actor|ActorHasTag (.hitactor _outhit) "Pickup")
            (bind _itemtopickup (Class|BPICombat|ScanItem(Message) (.hitactor _outhit)))
            (Utilities|IsValid _itemtopickup
              (:Is%20Valid
                (if (>= (Variables|Default|GetMoney) (.moneycost (Variables|/Game/Pickups/BP_BasePickup.BP_BasePickup_C|GetCurrentData _itemtopickup)))
                  (bind _output_get_2 (Variables|Default|SetMoney (- (Variables|Default|GetMoney) (.moneycost (Variables|/Game/Pickups/BP_BasePickup.BP_BasePickup_C|GetCurrentData _itemtopickup)))))
                  (Default|IncrementScore _timerbp_2 (.scorevalue (Variables|/Game/Pickups/BP_BasePickup.BP_BasePickup_C|GetCurrentData _itemtopickup)))
                  (Audio|PlaySound2D "/Game/Sound/SFX/SFX_ScanBarcode.SFX_ScanBarcode" 1.0 1.0 0.0 0 0)
                  (Default|UpdateDollarsValue (Variables|/Game/GMTK-2026/Blueprints/BP_PointTimer_Manager.BP_PointTimer_Manager_C|GetHUD_WBP _timerbp_2) _output_get_2))))
            (elif (Actor|ActorHasTag (.hitactor _outhit) "Enemy")
              (bind _enemyscanned (Class|BPICombat|ReturnEnemyBP(Message) (.hitactor _outhit)))
              (if (and (Variables|/Game/GMTK-2026/Blueprints/Enemies/BP_Base_Enemy.BP_Base_Enemy_C|GetStunned? _enemyscanned) (not (Variables|/Game/GMTK-2026/Blueprints/Enemies/BP_Base_Enemy.BP_Base_Enemy_C|GetbIsDying _enemyscanned)))
                (Class|BPICombat|ScanItem(Message) _enemyscanned)
                (Audio|PlaySound2D "/Game/Sound/SFX/SFX_ScanBarcode.SFX_ScanBarcode" 1.0 1.0 0.0 0 0)
                (Default|IncrementScore _timerbp (.scannedscore (Variables|/Game/GMTK-2026/Blueprints/Enemies/BP_Base_Enemy.BP_Base_Enemy_C|GetCurrentData _enemyscanned)))
                (bind _output_get_3 (Variables|Default|SetMoney (+ (Variables|Default|GetMoney) (/ (.dollarstakenonhit (Variables|/Game/GMTK-2026/Blueprints/Enemies/BP_Base_Enemy.BP_Base_Enemy_C|GetCurrentData _enemyscanned)) 2.0))))
                (Default|UpdateDollarsValue (Variables|/Game/GMTK-2026/Blueprints/BP_PointTimer_Manager.BP_PointTimer_Manager_C|GetHUD_WBP _timerbp) _output_get_3))))))))
  (:Started
    (if (not (Variables|Default|GetStunned?))
      (CallFunction|PlayFlipbook (Variables|Default|GetScanAnim))
      ;;;[0.15 0.15 0.15 0.5] Update Speed based on scanning
      (Variables|Default|SetScanning? true)
      (CallFunction|UpdateMovementSpeed (Variables|Default|GetScanningWalkSpeed))
      ;;;[0.15 0.15 0.15 0.5] Set flipbook playback speed
      (if _returnvalue
        (Components|Timeline|SetPlayRate _sprite 0.2)
        (else
          (Components|Timeline|SetPlayRate _sprite 0.4 :!label _label)))))
  (:Canceled
    (CallFunction|StopandHideFlipbook (Variables|Default|GetScanAnim) :!label _label_2)
    (Variables|Default|SetScanning? false)
    (CallFunction|UpdateMovementSpeed (Variables|Default|GetDefaultWalkSpeed))
    (if _returnvalue
      (goto _label)
      (else
        (goto _label))))
  (:Completed
    (goto _label_2)))

(event Input|EnhancedActionEvents|EnhancedInputActionIA_Shoot
  (params (ActionValue :type Boolean) (ElapsedSeconds :type Float%20%28double-precision%29) (TriggeredSeconds :type Float%20%28double-precision%29) (InputAction :type Input%20Action%20Object%20Reference :default "/Game/GMTK-2026/Input/Actions/IA_Shoot.IA_Shoot"))
  ;[0.15 0.15 0.15 0.5 50] Input Actions
  ;;[0.15 0.15 0.15 0.5] Shooting
  (if (and (> (- (Utilities|Time|GetGameTimeinSeconds) (Variables|Default|GetTimeSinceLastShot)) (Variables|Default|GetTimeBetweenShots)) (not (Variables|Default|GetStunned?)))
    (Variables|Default|SetTimeSinceLastShot (Utilities|Time|GetGameTimeinSeconds))
    (CallFunction|FireLaserBullt)
    (Audio|PlaySound2D "/Game/Sound/SFX/SFX_ShootLaser.SFX_ShootLaser" 1.0 (Math|Random|RandomFloatinRange 0.9 1.1) 0.0 0 0)))

(event EventBeginPlay
  ;[0.02718 1 0 0.5 50] Begin Play
  ;;[0.15 0.15 0.15 0.5] Temporary maybe? just wanted to test the scoring BP
  (bind _returnvalue (Actor|GetActorOfClass "/Game/GMTK-2026/Blueprints/BP_PointTimer_Manager.BP_PointTimer_Manager_C"))
  (Variables|Default|SetTimerBP _returnvalue)
  ;;[0.15 0.15 0.15 0.5] Allows Us To Fully Control The Spring Arm Pos
  (Transformation|DetachFromComponent (Variables|Default|GetSpringArm) "KeepWorld" "KeepWorld" "KeepWorld" true)
  (CallFunction|InitializeScanAnim)
  (EventDispatchers|AssignOnFinishedPlaying (Variables|Default|GetScanAnim) (delegate Custom|ScanAnimFinished))
  (CallFunction|UpdateMovementSpeed (Variables|Default|GetDefaultWalkSpeed))
  (bind _returnvalue_2 (Actor|GetActorOfClass "/Game/GMTK-2026/Blueprints/BP_ObjectPool.BP_ObjectPool_C"))
  (Variables|Default|SetObjectPooler _returnvalue_2)
  (Utilities|FlowControl|Delay 0.05)
  (Default|UpdateDollarsValue (Variables|/Game/GMTK-2026/Blueprints/BP_PointTimer_Manager.BP_PointTimer_Manager_C|GetHUD_WBP (Variables|Default|GetTimerBP)) (Variables|Default|GetMoney)))

(event EventTick
  (params (DeltaSeconds :type Float%20%28single-precision%29))
  (bind _returnvalue (Game|GetPlayerController 0))
  (bind _returnvalue_2 (Game|GetPlayerController 0))
  (bind _scannerspringarm (Variables|Default|GetScannerSpringArm))
  (bind _timerbp (Variables|Default|GetTimerBP))
  (bind _springarm (Variables|Default|GetSpringArm))
  (bind _hitresult (Game|Player|GetHitResultUnderCursorbyChannel _returnvalue "TraceTypeQuery2" true))
  (bind _returnvalue_3 (Transformation|GetWorldRotation _scannerspringarm))
  (bind (_hitresult_2 _returnvalue_4) (Game|Player|GetHitResultUnderCursorbyChannel _returnvalue_2 "TraceTypeQuery3" true))
  (bind _hud_wbp (Variables|/Game/GMTK-2026/Blueprints/BP_PointTimer_Manager.BP_PointTimer_Manager_C|GetHUD_WBP _timerbp))
  (bind _location (Collision|BreakHitResult _hitresult_2))
  (bind (_bblockinghit _binitialoverlap _time _distance _location_2 _impactpoint _normal _impactnormal _physmat _hitactor) (Collision|BreakHitResult _hitresult))
  ;[0.02718 1 0 0.5 50] Tick
  (Variables|Default|SetDelta%20Seconds DeltaSeconds)
  (Utilities|FlowControl|Sequence
    (:then_0
      (CallFunction|DetermineCurrentAnimState))
    (:then_1
      ;;[0.02718 1 0 0.5 30] Camera Movement
      (Variables|Default|SetCursorLocation _location)
      (Variables|Default|SetisCursorInValidRegion _returnvalue_4)
      (Utilities|FlowControl|Sequence
        (:then_0
          (if (Variables|Default|GetisCursorInValidRegion)
            ;;[0.02718 1 0 0.5 30] Rotate Scanner Hand
            (Transformation|SetWorldRotation _scannerspringarm (Math|Rotator|MakeRotator (.roll _returnvalue_3) (.pitch _returnvalue_3) (+ (.yaw (Math|Rotator|FindLookatRotation (Transformation|GetWorldLocation (Variables|Default|GetScannerSpringArm)) _location)) -1.8e+02)) false false)))
        (:then_1
          (if (Variables|Default|GetisCursorInValidRegion)
            (bind (_returnvalue_x _returnvalue_y) (CallFunction|CalculateCameraOffset))
            (Transformation|SetWorldLocation (Variables|Default|GetSpringArm) (Math|Interpolation|VInterpTo (Transformation|GetWorldLocation _springarm) (Math|Vector|MakeVector _returnvalue_x _returnvalue_y (.z (Transformation|GetWorldLocation _springarm))) (Variables|Default|GetDelta%20Seconds) (Variables|Default|GetCameraFollowSpeed)) false false)))
        (:then_2
          ;[0.15 0.15 0.15 0.5] LiveDataFeed
          (if _bblockinghit
            (if (Utilities|DoesObjectImplementInterface _hitactor "/Game/GMTK-2026/Blueprints/BPI_Combat.BPI_Combat_C")
              (bind (_pickupdeets _enemydeets) (Class|BPICombat|ReturnStruct(Message) _hitactor))
              (if (Utilities|Enum|NotEqual(Enum) (.itemname _pickupdeets) "")
                (Default|UpdateFocusedItemDetails _hud_wbp (.itemname _pickupdeets) (Utilities|String|Append "Score Value : " (Utilities|String|ToString(Integer) (.scorevalue _pickupdeets))) (Utilities|String|Append "Cost : " (Utilities|String|ToString(Float) (.moneycost _pickupdeets))))
                (elif (Utilities|Enum|NotEqual(Enum) (.enemyname _enemydeets) "")
                  (Default|UpdateFocusedItemDetails _hud_wbp (.enemyname _enemydeets) (Utilities|String|Append "Score Value : " (Utilities|String|ToString(Integer) (.scannedscore _enemydeets))) (Utilities|String|Append "$$$ : " (Utilities|String|ToString(Float) (.dollarstakenonhit _enemydeets))))))
              (else
                (Default|CloseFocusUI (Variables|/Game/GMTK-2026/Blueprints/BP_PointTimer_Manager.BP_PointTimer_Manager_C|GetHUD_WBP (Variables|Default|GetTimerBP)))))))))))

(event EventSendHit
  (params (Direction :type Vector :default "0, 0, 0") (DollarsTaken :type Float%20%28double-precision%29))
  (bind _timerbp (Variables|Default|GetTimerBP))
  (bind _hud_wbp (Variables|/Game/GMTK-2026/Blueprints/BP_PointTimer_Manager.BP_PointTimer_Manager_C|GetHUD_WBP _timerbp))
  ;[0.15 0.15 0.15 0.5 50] Temporary
  ;;[1 0 0 0.5] Getting hit by enemies
  (CallFunction|Knockback Direction)
  (if (<= (- (Variables|Default|GetMoney) DollarsTaken) 0.0)
    (Variables|Default|SetMoney 0.0)
    (Default|UpdateDollarsValue _hud_wbp 0.0)
    (else
      (bind _output_get (Variables|Default|SetMoney (- (Variables|Default|GetMoney) DollarsTaken)))
      (Default|UpdateDollarsValue _hud_wbp _output_get))))

(event Input|KeyboardEvents|DebugKeyC
  (params (Key :type Key%20Structure :default "None") (ActionValue :type Input%20Action%20Value%20Structure)))

(event Input|KeyboardEvents|LeftCtrl
  (params (Key :type Key%20Structure :default "None"))
  ;[0.15 0.15 0.15 0.5 50] Temporary
  ;;[1 0 0 0.5] Definetely temporary
  (:Pressed
    (Default|IncrementScore (Variables|Default|GetTimerBP))))

(fn ConstructionScript
  (Variables|Default|SetStartingScale (Variables|/Script/Engine.SceneComponent|GetRelativeScale3D (Variables|Default|GetSprite))))

(fn CalculateCameraOffset
  (bind _returnvalue (Transformation|GetActorLocation))
  (bind _returnvalue_2 (Transformation|GetActorLocation))
  (bind _cameraoffsetstrength (Variables|Default|GetCameraOffsetStrength))
  (bind _cursorlocation (Variables|Default|GetCursorLocation))
  (bind _returnvalue_3 (- _cursorlocation _returnvalue))
  (bind _returnvalue_4 (* _returnvalue_3 _cameraoffsetstrength))
  (bind _returnvalue_5 (+ _returnvalue_2 _returnvalue_4))
  (return (.x _returnvalue_5) (.y _returnvalue_5)))

(fn InitializeScanAnim
  (bind _scananim (Variables|Default|GetScanAnim))
  (Audio|Components|Audio|Stop _scananim)
  (Development|SetHiddeninGame _scananim true false)
  (Components|Timeline|SetPlayRate _scananim (Variables|Default|GetScannerAnimPlaybackRate)))

(fn StopandHideFlipbook
  (params (Flipbook :type Paper%20Flipbook%20Component%20Object%20Reference))
  (Audio|Components|Audio|Stop Flipbook)
  (Development|SetHiddeninGame Flipbook true false))

(fn PlayFlipbook
  (params (Flipbook :type Paper%20Flipbook%20Component%20Object%20Reference))
  (Development|SetHiddeninGame Flipbook false false)
  (Components|Timeline|PlayfromStart Flipbook))

(fn CalculateShotStartingPos
  (return (+ (.location (Transformation|GetActorTransform (Game|GetPlayerCharacter 0))) (* (Math|Vector|GetForwardVector (Variables|Default|GetScannerHand)) (Math|Conversions|ToVector(Float) (Variables|Default|GetScanColliderStartOffset))))))

(fn CalculateSphereTraceEnd
  (return (+ (.location (Transformation|GetActorTransform (Game|GetPlayerCharacter 0))) (* (Math|Vector|GetForwardVector (Variables|Default|GetScannerHand)) (Math|Conversions|ToVector(Float) (Variables|Default|GetScanColliderDistance))))))

(fn UpdateMovementSpeed
  (params (Desired%20Speed :type Float%20%28double-precision%29))
  (if (not (Variables|Default|GetSpeedBoostActive))
    (Variables|/Script/Engine.CharacterMovementComponent|SetMaxWalkSpeed (Variables|Character|GetCharacterMovement) Desired%20Speed)
    (else
      (Variables|/Script/Engine.CharacterMovementComponent|SetMaxWalkSpeed (Variables|Character|GetCharacterMovement) (* Desired%20Speed (Variables|Default|GetSpeedBoostModifier))))))

(fn FireLaserBullt
  (bind _spheretracestart (CallFunction|CalculateShotStartingPos))
  (Default|GetPooledActor (Variables|Default|GetObjectPooler) "NewEnumerator0" (+ _spheretracestart (* (Math|Vector|GetForwardVector (Variables|Default|GetScannerHand)) 15)) (Transformation|GetWorldRotation (Variables|Default|GetScannerHand)) true))

(fn ReturnEnemyBP
  (return 0))

(fn ReturnPlayerRef
  (return self))

(fn ReturnStruct
  (return "" ""))

(fn ScanItem
  (return 0))