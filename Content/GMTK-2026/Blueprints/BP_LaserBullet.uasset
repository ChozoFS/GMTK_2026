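; BP_LaserBullet is a pooled laser projectile that delivers hit messages to combat-capable actors it overlaps.
; On activation from the pool it sets its projectile movement velocity along its forward vector and starts a timer that recycles it through its AC_PooledObject component.
; Capsule overlaps send a hit message to actors implementing BPI_Combat, without recycling the bullet, so it keeps flying until the timer fires.
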(event `self.ReceiveBeginPlay`)

(event `self.Capsule.OnComponentBeginOverlap`
  (params (OverlappedComponent :type "PrimitiveComponent Object Reference") (OtherActor :type "Actor Object Reference") (OtherComp :type "PrimitiveComponent Object Reference") (OtherBodyIndex :type Integer) (bFromSweep :type Boolean) (SweepResult :type "HitResult Structure (by ref)"))
  (if (`KismetSystemLibrary.DoesImplementInterface` OtherActor "/Game/GMTK-2026/Blueprints/BPI_Combat.BPI_Combat_C")
    (message `/Game/GMTK-2026/Blueprints/BPI_Combat.SendHit` OtherActor)))

(event `/Game/GMTK-2026/Blueprints/BPI_Poolable.OnActivatedFromPool`
  (set `MovementComponent.Velocity` (* (`self.GetActorForwardVector`) (`self.ProjectileSpeed`)) (`self.ProjectileMovement`))
  (`KismetSystemLibrary.K2_SetTimerDelegate` (delegate `RecycleToPool`) 3.0))

(event `RecycleToPool`
  (bind _returnvalue (`self.GetComponentByClass` "/Game/GMTK-2026/Blueprints/AC_PooledObject.AC_PooledObject_C"))
  (`/Engine/EditorBlueprintResources/StandardMacros.IsValid` _returnvalue
    (:`Is Valid`
      (`/Game/GMTK-2026/Blueprints/AC_PooledObject.RecycleSelf` _returnvalue))))

(fn `UserConstructionScript`)