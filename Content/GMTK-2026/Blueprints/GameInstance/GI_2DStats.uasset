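; Game instance that keeps the scores of three levels and totals them into a final score.
; The PassLevelResults event stores an incoming score in the variable matching its level number.
; ReturnFinalScores sums the three stored scores, and PassFinalScores relays the total along with each level score.
; PassGameInstanceOb returns a reference to the instance itself.
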(event `/Game/GMTK-2026/Blueprints/GameInstance/BPI_GameInstance.PassLevelResults`
  (params (Level :type Integer) (Score :type Integer))
  (switch `int` Level
    (:`1`
      (set `self.LevelScore_01` Score))
    (:`2`
      (set `self.LevelScore_02` Score))
    (:`3`
      (set `self.LevelScore_03` Score))))

(fn `PassFinalScores`
  (returns (ScoreLevel_01 :type Integer) (ScoreLevel_02 :type Integer) (ScoreLevel_03 :type Integer) (FinalScore :type Integer))
  (bind (_finalscore _levelscore_01 _levelscore_02 _levelscore_03) (`self.ReturnFinalScores`))
  (return _levelscore_01 _levelscore_02 _levelscore_03 _finalscore))

(fn `PassGameInstanceOb`
  (returns (ThisGameInstance :type "/Game/GMTK-2026/Blueprints/GameInstance/GI_2DStats Object Reference"))
  (return self))

(fn `ReturnFinalScores`
  (returns (FinalScore :type Integer) (LevelScore_01 :type Integer) (LevelScore_02 :type Integer) (LevelScore_03 :type Integer))
  (bind _levelscore_01 (`self.LevelScore_01`))
  (bind _levelscore_02 (`self.LevelScore_02`))
  (bind _levelscore_03 (`self.LevelScore_03`))
  (bind _output_get (set `self.Finalscore` (+ _levelscore_01 _levelscore_02 _levelscore_03)))
  (return _output_get _levelscore_01 _levelscore_02 _levelscore_03))