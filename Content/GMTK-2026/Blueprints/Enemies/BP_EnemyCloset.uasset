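; Enemy closet spawner that creates a randomly chosen enemy at a fixed point whenever SpawnChosenUnit is called.
; BeginPlay caches the world position of its SPAWNLOCATION component, which ReturnSpawnLocation also exposes.
; SpawnChosenUnit always spawns an EnemyClass actor there, ignoring collisions, then passes it a DT_Enemies row via AssumeIdentity.
; ChooseUnitToSpawn picks that row at random from SpawnableEnemies, so enemy variety is data-driven.
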(event `self.ReceiveBeginPlay`
  (set `self.WorldSpawnLocation` (`SceneComponent.K2_GetComponentLocation` (`self.SPAWNLOCATION`))))

(event `SpawnChosenUnit`
  (`KismetSystemLibrary.PrintString` "Spawn attempt")
  (bind _returnvalue (`|SpawnActorFromClass` (`self.EnemyClass`) (`KismetMathLibrary.MakeTransform` (`self.WorldSpawnLocation`)) "AlwaysSpawn" "MultiplyWithRoot" null null))
  (bind _enemydetails (`self.ChooseUnitToSpawn`))
  (`/Game/GMTK-2026/Blueprints/Enemies/BP_Base_Enemy.AssumeIdentity` _returnvalue _enemydetails))

(fn `ChooseUnitToSpawn`
  (returns (EnemyDetails :type "/Game/GMTK-2026/Blueprints/Enemies/Struct_EnemyDetails Structure"))
  (bind _returnvalue (`|GetDataTableRow` "/Game/GMTK-2026/Blueprints/Enemies/DT_Enemies.DT_Enemies" (`.RowName` (break `DataTableRowHandle` (`KismetArrayLibrary.Array_Random` (`self.SpawnableEnemies`)))))
    (:`then`
      (return _returnvalue))))

(fn `ReturnSpawnLocation`
  (returns (SpawnLocationHere :type "Vector Structure"))
  (return (`self.WorldSpawnLocation`)))

(fn `UserConstructionScript`)