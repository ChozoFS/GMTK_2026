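; Enemy spawn manager that periodically triggers enemy spawns from a set of managed closets.
; From BeginPlay it runs an endless loop: wait a random interval between the min and max settings, pick a random closet, call its SpawnChosenUnit, then wait again.
; A debug print announces the wait, but it rolls its own random value, so the displayed time can differ from the actual delay.
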(event `self.ReceiveBeginPlay`
  (`self.BeginWaitWindow`))

(event `BeginWaitWindow`
  (bind _returnvalue (`KismetMathLibrary.RandomFloatInRange` (`self.MinSpawnInterval`) (`self.MaxSpawnInterval`)))
  (`KismetSystemLibrary.PrintString` (`KismetStringLibrary.Concat_StrStr` "SPAWNING IN : " (`KismetStringLibrary.Conv_DoubleToString` _returnvalue) " Seconds") true true (struct :`R` 1.0 :`G` 0.962762 :`A` 1.0) 5.0)
  (`KismetSystemLibrary.Delay` _returnvalue)
  (`self.SpawnUnit`))

(event `SpawnUnit`
  (bind _closettospawnfrom (`self.ChooseCloset`))
  (`/Game/GMTK-2026/Blueprints/Enemies/BP_EnemyCloset.SpawnChosenUnit` _closettospawnfrom)
  (`self.BeginWaitWindow`))

(fn `ChooseCloset`
  (returns (ClosetToSpawnFrom :type "/Game/GMTK-2026/Blueprints/Enemies/BP_EnemyCloset Object Reference"))
  (return (`KismetArrayLibrary.Array_Random` (`self.ClosetsToManage`))))

(fn `UserConstructionScript`)