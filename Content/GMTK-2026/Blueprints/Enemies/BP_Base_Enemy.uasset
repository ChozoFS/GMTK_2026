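; Base 2D flipbook enemy character that players stun with hits, then destroy by scanning.
; AssumeIdentity applies a data struct for name, sprite, tint, speed and score.
; SendHit launches and freezes it on a retriggerable timer with a pooled stun effect and scan indicator; scanning then triggers a flash, burst and destruction.
; Hitbox overlap sends the player a hit message; movement AI and hit re-arming are unwired.
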(event `self.ReceiveBeginPlay`
  (set `self.PlayerPawn` (`Controller.K2_GetPawn` (`GameplayStatics.GetPlayerController` 0)))
  (bind _returnvalue (`GameplayStatics.GetActorOfClass` "/Game/GMTK-2026/Blueprints/BP_ObjectPool.BP_ObjectPool_C"))
  (set `self.ObjectPooler` _returnvalue))

(event `HuntPlayer`)

(event `self.HitBox.OnComponentBeginOverlap`
  (params (OverlappedComponent :type "PrimitiveComponent Object Reference") (OtherActor :type "Actor Object Reference") (OtherComp :type "PrimitiveComponent Object Reference") (OtherBodyIndex :type Integer) (bFromSweep :type Boolean) (SweepResult :type "HitResult Structure (by ref)"))
  (if (`self.ActorHasTag` OtherActor "Player")
    (bind _output_get (set `self.Other Actor` OtherActor))
    (if (`self.CanHit`)
      (message `/Game/GMTK-2026/Blueprints/BPI_Combat.SendHit` _output_get (0.0 0.0 0.0))
      (set `self.CanHit` false))))

(event `self.HitBox.OnComponentEndOverlap`
  (params (OverlappedComponent :type "PrimitiveComponent Object Reference") (OtherActor :type "Actor Object Reference") (OtherComp :type "PrimitiveComponent Object Reference") (OtherBodyIndex :type Integer))
  (if (`self.ActorHasTag` OtherActor "Player")
    (set `self.Other Actor` null)))

(event `/Game/GMTK-2026/Blueprints/BPI_Combat.SendHit`
  (params (Direction :type "Vector Structure"))
  (bind (_returnvalue_x _returnvalue_y) (`KismetMathLibrary.BreakVector` (* Direction 1500.0)))
  (bind (_currentdata_enemyname _currentdata_defaultspriteanim _currentdata_movementspeed) (break `/Game/GMTK-2026/Blueprints/Enemies/Struct_EnemyDetails` (`self.CurrentData`)))
  ; Knockback/stun on projectile hit
  (if (not (`self.StunVFX Playing?`))
    (bind _pooledactor (`/Game/GMTK-2026/Blueprints/BP_ObjectPool.GetPooledActor` :`self` (`self.ObjectPooler`) :`Object Type` "NewEnumerator1" :`DesiredSpawnLocation` (`SceneComponent.K2_GetComponentLocation` (`self.StunVFXSpawnPoint`)) :`UseCustomSpawnLocationAndRotation` true))
    (`self.K2_AttachToActor` _pooledactor self "None" "SnapToTarget" "SnapToTarget" "KeepRelative" true)
    (set `self.StunVFX Playing?` true))
  (set `self.Stunned?` true)
  (`self.LaunchCharacter` (`KismetMathLibrary.MakeVector` _returnvalue_x _returnvalue_y 10.0) true true)
  (set `CharacterMovementComponent.MaxWalkSpeed` 0.0 (`self.CharacterMovement`))
  (`SceneComponent.SetVisibility` (`self.SPR_ScanIndicator_Sprite`) true false)
  (`KismetSystemLibrary.RetriggerableDelay` 3.0)
  (`/Game/GMTK-2026/Blueprints/BP_ObjectPool.RecycleActor` (`self.ObjectPooler`) _pooledactor)
  (set `self.StunVFX Playing?` false)
  (set `self.Stunned?` false)
  (set `CharacterMovementComponent.MaxWalkSpeed` _currentdata_movementspeed (`self.CharacterMovement`))
  (`SceneComponent.SetVisibility` (`self.SPR_ScanIndicator_Sprite`) false false))

(event `Scan`
  (bind _scanflash (`self.ScanFlash`))
  ; Kill on Scan
  (if (`self.Stunned?`)
    (`/Engine/EditorBlueprintResources/StandardMacros.DoOnce` false
      (:`Completed`
        (set `self.bIsDying` true)
        (`SceneComponent.SetVisibility` _scanflash true false)
        (`PaperFlipbookComponent.SetPlayRate` _scanflash 1.0)
        (`KismetSystemLibrary.Delay` 0.36)
        (`NiagaraFunctionLibrary.SpawnSystemAtLocation` "/Game/GMTK-2026/FX/Scan/NE_ScanBurst.NE_ScanBurst" (`SceneComponent.K2_GetComponentLocation` (`self.CapsuleComponent`)))
        (`KismetSystemLibrary.PrintString` "KABOOOOM" true true (struct :`R` 0.142012 :`G` 1.0 :`A` 1.0))
        (`SceneComponent.SetVisibility` (`self.ScanFlash`) false false)
        (`GameplayStatics.PlaySound2D` "/Game/Sound/SFX/SFX_ScanExplode.SFX_ScanExplode" 1.0 (`KismetMathLibrary.RandomFloatInRange` 0.9 1.1) 0.0 null null)
        ; feel free to unplug once pooling is in
        (`self.K2_DestroyActor`)))))

(event `AssumeIdentity`
  (params (NewData :type "/Game/GMTK-2026/Blueprints/Enemies/Struct_EnemyDetails Structure"))
  (bind _paperflipbook (`self.PaperFlipbook`))
  ;[0.2498 0.2522 0.08473] SETTING UNITS Data
  (bind _output_get (set `self.CurrentData` NewData))
  (`KismetSystemLibrary.PrintString` "IDENTITY")
  (bind (_enemyname _defaultspriteanim _movementspeed _spritetint _score) (break `/Game/GMTK-2026/Blueprints/Enemies/Struct_EnemyDetails` _output_get))
  (set `self.MyCurrentName` _enemyname)
  (`PaperFlipbookComponent.SetFlipbook` _paperflipbook _defaultspriteanim)
  (set `CharacterMovementComponent.MaxWalkSpeed` _movementspeed (`self.CharacterMovement`))
  (`PaperFlipbookComponent.SetSpriteColor` _paperflipbook _spritetint)
  (set `self.MyScoreValue` _score))

(fn `ReturnEnemyBP`
  (returns (EnemyScanned :type "/Game/GMTK-2026/Blueprints/Enemies/BP_Base_Enemy Object Reference"))
  (return self))

(fn `ReturnPlayerRef`
  (returns (Player :type "/Game/GMTK-2026/Blueprints/BP_Character2D Object Reference"))
  (return null))

(fn `ReturnStruct`
  (returns (PickupDeets :type "/Game/Pickups/Struct_Pickup Structure") (EnemyDeets :type "/Game/GMTK-2026/Blueprints/Enemies/Struct_EnemyDetails Structure"))
  (return (struct) (`self.CurrentData`)))

(fn `ScanItem`
  (returns (ItemToPickup :type "/Game/Pickups/BP_BasePickup Object Reference"))
  (`self.Scan`)
  (return null))

(fn `UserConstructionScript`)